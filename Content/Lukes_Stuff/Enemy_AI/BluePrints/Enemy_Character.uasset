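; Enemy character that chases the player using AI MoveTo toward the player character.
; Tick, BeginPlay and PawnSensing's OnSeePawn share one check that calls FollowPlayer while Playing is true.
; Seeing a pawn also sets IsSeeingPlayer, but the chase does not depend on it.
; The overlap event checks for the player pawn but takes no action.
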(event OnSeePawn(PawnSensing)
  (params (Pawn :type Pawn%20Object%20Reference))
  ;[1 1 1] Follow
  (Variables|Default|SetIs_Seeing_Player true)
  (if (Variables|Default|GetPlaying)
    (CallFunction|FollowPlayer)))

(event Custom|FollowPlayer
  ;[1 1 1] Follow
  (AI|AIMoveTo self "0, 0, 0" (Game|GetPlayerCharacter 0) 17.0 false))

(event EventTick
  (params (DeltaSeconds :type Float%20%28single-precision%29))
  ;[1 1 1] Follow
  (if (Variables|Default|GetPlaying)
    (CallFunction|FollowPlayer)))

(event EventBeginPlay
  ;[1 1 1] Follow
  (if (Variables|Default|GetPlaying)
    (CallFunction|FollowPlayer)))

(event Collision|EventActorBeginOverlap
  (params (OtherActor :type Actor%20Object%20Reference))
  ;[1 1 1] Overlap
  (if (== OtherActor (Game|Player|GetPlayerPawn 0))
    _))

(fn ConstructionScript)