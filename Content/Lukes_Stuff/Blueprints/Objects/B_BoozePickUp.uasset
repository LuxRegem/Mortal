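; Booze pickup that hides itself when the drinking first-person player's Pickup event fires, then respawns.
; On BeginPlay it binds HideBooze to that event on player 0's character, with no check in this Blueprint for which pickup was collected.
; HideBooze turns off the box's overlap events and hides the mesh, then restores both after a six-second delay.
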(event Custom|HideBooze
  (bind _self self)
  (bind _boxoverlap (Variables|Default|GetBoxOverlap _self))
  (bind _mesh (Variables|Default|GetMesh _self))
  (Variables|/Script/Engine.PrimitiveComponent|SetbGenerateOverlapEvents _boxoverlap false)
  (Rendering|SetVisibility _mesh false false)
  (Utilities|FlowControl|Delay 6.0)
  (Variables|/Script/Engine.PrimitiveComponent|SetbGenerateOverlapEvents _boxoverlap true)
  (Rendering|SetVisibility _mesh true false))

(event EventBeginPlay
  (EventDispatchers|BindEventtoPickup (.AsBP%20Drinking%20First%20Person%20Character (Utilities|Casting|CastToBP_DrinkingFirstPersonCharacter (Game|Player|GetPlayerPawn 0))) (delegate Custom|HideBooze)))

(event EventTick
  (params (DeltaSeconds :type Float%20%28single-precision%29)))

(fn ConstructionScript)